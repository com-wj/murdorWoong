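; Interactive keypad that blends the view to its camera and lets the player click in a fixed or random code.
; F, right mouse or Interact toggles use, swapping player input and cursor.
; Clicks trace tagged key components, animate them and use their object names as digit, Clear or Enter.
; EnterCode flashes a green or red light with a buzzer; success zooms out and applies tiny self-damage, while door-unlock logic is unconnected.
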(event `AnimateKey`
  ;[1 1 1] 키 이동을 애니메이션합니다. 먼저 버튼의 상대 위치를 가져와 누르고 있는 버튼을 애니메이션합니다.
  (if (not (`self.AnimationPlaying?`))
    (bind _output_get (set `self.StartLocation` (`SceneComponent.RelativeLocation` (`self.ClickedKey`))))
    (set `self.EndLocation` (`KismetMathLibrary.MakeVector` (.x _output_get) -0.1 (.z _output_get)))
    (bind (_direction _pressanimation) (`Timeline|AnimateKeyPress` :!via `PlayFromStart`)
      (:`Update`
        (`SceneComponent.K2_SetRelativeLocation` (`self.ClickedKey`) (`KismetMathLibrary.VLerp` (`self.StartLocation`) (`self.EndLocation`) _pressanimation) false false)
        (set `self.AnimationPlaying?` true))
      (:`Finished`
        (set `self.AnimationPlaying?` false)))))

(event `self.ReceiveTick`
  (params (DeltaSeconds :type "Float (single-precision)"))
  (bind _returnvalue (`GameplayStatics.GetPlayerController` 0))
  ;[1 1 1] 이벤트 틱. 플레이어가 사용하는 동안 키패드에 대한 입력을 활성화합니다.
  (if (`self.UsingKeypad?`)
    (`self.EnableInput` _returnvalue)
    (`WidgetBlueprintLibrary.SetInputMode_GameOnly` _returnvalue)
    (else
      (`self.DisableInput` _returnvalue))))

(event `Key|LeftMouseButton`
  (params (Key :type "Key Structure"))
  (bind (_hitresult _returnvalue) (`PlayerController.GetHitResultUnderCursorForObjects` (`GameplayStatics.GetPlayerController` 0) (`|MakeArray` "ObjectTypeQuery1" "ObjectTypeQuery2" :!type "EObjectTypeQuery Enum") true))
  (bind _returnvalue_2 (`SceneComponent.K2_GetComponentLocation` (`self.Keypad`)))
  (bind (_bblockinghit _binitialoverlap _time _distance _location _impactpoint _normal _impactnormal _physmat _hitactor _hitcomponent) (`GameplayStatics.BreakHitResult` _hitresult))
  (bind _returnvalue_3 (`KismetSystemLibrary.GetObjectName` _hitcomponent))
  ;[1 1 1] 플레이어가 버튼을 클릭할 때 호출됩니다. 눌려진 버튼을 찾은 다음 코드를 입력하거나 입력한 코드를 지우거나 배열에 숫자를 추가합니다.
  (:`Pressed`
    (if (and _returnvalue (`ActorComponent.ComponentHasTag` _hitcomponent "Key"))
      (set `self.ClickedKey` _hitcomponent)
      (`self.AnimateKey`)
      (`GameplayStatics.PlaySoundAtLocation` (`self.KeyPressSoundCue`) (`SceneComponent.K2_GetComponentLocation` (`self.Keypad`)) (struct) 1.0 1.0 0.0 null null null)
      (switch `string` _returnvalue_3
        (:`Default`
          (`KismetArrayLibrary.Array_Add` (`self.EnteredCode`) (`KismetStringLibrary.Conv_StringToInt` _returnvalue_3))
          (if (and (== (`KismetArrayLibrary.Array_Length` (`self.EnteredCode`)) (`self.CodeLength`)) (`self.AutomaticallyEnderCode`))
            (for _array_element (`self.EnteredCode`) :!label _label
              (set `self.CodeString` (`KismetStringLibrary.Concat_StrStr` (`self.CodeString`) (`KismetStringLibrary.Conv_IntToString` _array_element))))
            (if (and (`KismetStringLibrary.EqualEqual_StrStr` (`self.Code`) (`self.CodeString`)) (<= (`KismetArrayLibrary.Array_Length` (`self.EnteredCode`)) (`self.CodeLength`)))
              (`self.ClearCode`)
              (`PrimitiveComponent.SetMaterial` (`self.Keypad`) 0 (`self.KeypadMaterialRight`))
              (`KismetSystemLibrary.Delay` 0.2)
              (`MaterialInstanceDynamic.SetScalarParameterValue` (`self.KeypadMaterialRight`) "Emmisivestrength" 150.0)
              (`GameplayStatics.PlaySoundAtLocation` (`self.BuzzerRightSoundCue`) _returnvalue_2 (struct) 1.0 1.0 0.0 null null null)
              (`KismetSystemLibrary.Delay` 0.54)
              (`MaterialInstanceDynamic.SetScalarParameterValue` (`self.KeypadMaterialRight`) "Emmisivestrength" 0.0)
              (if (`self.CorrectCode?`)
                _
                (else
                  _))
              (set `self.CorrectCode?` true)
              (`self.CorrectCode_ZoomOut`)
              (else
                (`self.ClearCode`)
                (`PrimitiveComponent.SetMaterial` (`self.Keypad`) 0 (`self.KeypadMaterialWrong`))
                (`KismetSystemLibrary.Delay` 0.2)
                (`MaterialInstanceDynamic.SetScalarParameterValue` (`self.KeypadMaterialWrong`) "Emmisivestrength" 150.0)
                (`GameplayStatics.PlaySoundAtLocation` (`self.BuzzerWrongSoundCue`) _returnvalue_2 (struct) 1.0 1.0 0.0 null null null)
                (`KismetSystemLibrary.Delay` 0.54)
                (`MaterialInstanceDynamic.SetScalarParameterValue` (`self.KeypadMaterialWrong`) "Emmisivestrength" 0.0)
                (set `self.CorrectCode?` false)))
            (if (`self.CorrectCode?`)
              (`GameplayStatics.ApplyDamage` self 0.0001))))
        (:`Enter`
          (goto _label))
        (:`Clear`
          (`self.ClearCode`))))))

(event `CorrectCode_ZoomOut`
  (bind _returnvalue (`GameplayStatics.GetPlayerController` 0))
  ;[1 1 1] 플레이어가 키패드와 상호 작용하면 카메라가 가까이 확대되고 커서가 활성화됩니다. 이렇게 하면 플레이어가 버튼을 클릭할 수 있습니다. 같은 버튼을 다시 누르면 반대 현상이 발생합니다
  (`PlayerController.SetViewTargetWithBlend` (`GameplayStatics.GetPlayerController` 0) (`GameplayStatics.GetPlayerCharacter` 0) 1.0 "VTBlend_EaseIn" 1.2 false)
  (set `PlayerController.bShowMouseCursor` false (`GameplayStatics.GetPlayerController` 0) :!label _label_2)
  (`WidgetBlueprintLibrary.SetInputMode_GameOnly` _returnvalue)
  (bind _asgi_woong (cast `/Game/GI_Woong` (`GameplayStatics.GetGameInstance`)))
  (set `/Game/GI_Woong.mouse_CenterFocus` true _asgi_woong)
  (set `PlayerController.CurrentMouseCursor` "None" _returnvalue))

(event `Key|F`
  (params (Key :type "Key Structure"))
  (bind _returnvalue (`GameplayStatics.GetPlayerController` 0))
  ;[1 1 1] 플레이어가 키패드와 상호 작용하면 카메라가 가까이 확대되고 커서가 활성화됩니다. 이렇게 하면 플레이어가 버튼을 클릭할 수 있습니다. 같은 버튼을 다시 누르면 반대 현상이 발생합니다
  (:`Pressed`
    (`/Engine/EditorBlueprintResources/StandardMacros.DoOnce` false :!label _label_3
      (:`Completed`
        (`|ExecutionSequence`
          (:`then_0`
            (if (`self.UsingKeypad?`)
              (`self.ClearCode`)
              (set `self.UsingKeypad?` false)
              (`|ExecutionSequence`
                (:`then_0`
                  (`PlayerController.SetViewTargetWithBlend` (`GameplayStatics.GetPlayerController` 0) (`GameplayStatics.GetPlayerCharacter` 0) 0.4 "VTBlend_Linear" 0.0 false)
                  (goto _label_2))
                (:`then_1`
                  (`KismetSystemLibrary.Delay` 0.5)
                  (`self.Enable/DisablePlayerInput` true)))
              (else
                (set `self.UsingKeypad?` true)
                (`self.Enable/DisablePlayerInput` false)
                (`PlayerController.SetViewTargetWithBlend` (`GameplayStatics.GetPlayerController` 0) self 0.4 "VTBlend_Linear" 0.0 false)
                (bind _asgi_woong (cast `/Game/GI_Woong` (`GameplayStatics.GetGameInstance`)))
                (set `/Game/GI_Woong.mouse_CenterFocus` false _asgi_woong)
                (set `PlayerController.CurrentMouseCursor` "Default" _returnvalue)
                (set `PlayerController.bShowMouseCursor` true _returnvalue))))
          (:`then_1`
            (`KismetSystemLibrary.Delay` 0.7) ; 카메라 시점 변환 딜레이
            (goto _label_3 :!via `Reset`)))))))

(event `Key|RightMouseButton`
  (params (Key :type "Key Structure"))
  ;[1 1 1] 플레이어가 키패드와 상호 작용하면 카메라가 가까이 확대되고 커서가 활성화됩니다. 이렇게 하면 플레이어가 버튼을 클릭할 수 있습니다. 같은 버튼을 다시 누르면 반대 현상이 발생합니다
  (:`Pressed`
    (goto _label_3)))

(event `/Game/PadlockAndKeypadPack/Interfaces/BPI_Interact.Interact`
  ;[1 1 1] 플레이어가 키패드와 상호 작용하면 카메라가 가까이 확대되고 커서가 활성화됩니다. 이렇게 하면 플레이어가 버튼을 클릭할 수 있습니다. 같은 버튼을 다시 누르면 반대 현상이 발생합니다
  (goto _label_3))

(fn `ClearCode`
  ;[1 1 1] Resets the code when the clear button is pressed
  (`KismetArrayLibrary.Array_Clear` (`self.EnteredCode`))
  (set `self.CodeString` "")
  (return))

(fn `Enable/DisablePlayerInput`
  (params (`Enable?` :type Boolean))
  (if `Enable?`
    (`self.EnableInput` (`GameplayStatics.GetPlayerCharacter` 0) (`GameplayStatics.GetPlayerController` 0))
    (`self.DisableInput` (`GameplayStatics.GetPlayerController` 0))
    (else
      (`self.DisableInput` (`GameplayStatics.GetPlayerCharacter` 0) (`GameplayStatics.GetPlayerController` 0)))))

(fn `LineTraceForKeypad`
  (locals (TraceStartLocation :type "Vector Structure") (TraceEndLocation :type "Vector Structure"))
  (bind _returnvalue (`GameplayStatics.GetPlayerController` 0))
  (bind _output (`|GetArrayItem` (`self.K2_GetComponentsByClass` (`GameplayStatics.GetPlayerCharacter` 0) "/Script/Engine.CameraComponent")))
  (bind _returnvalue_2 (`SceneComponent.K2_GetComponentLocation` _output))
  (set `local.TraceStartLocation` _returnvalue_2)
  (set `local.TraceEndLocation` (+ _returnvalue_2 (* (`SceneComponent.GetForwardVector` _output) 250.0)))
  (set `self.ItemName` "")
  (bind (_outhit _returnvalue_3) (`KismetSystemLibrary.LineTraceSingle` :`Start` (`local.TraceStartLocation`) :`End` (`local.TraceEndLocation`) :`TraceChannel` "TraceTypeQuery1" :`bIgnoreSelf` false))
  (if _returnvalue_3
    (bind (_bblockinghit _binitialoverlap _time _distance _location _impactpoint _normal _impactnormal _physmat _hitactor _hitcomponent) (`GameplayStatics.BreakHitResult` _outhit))
    (if (and (`KismetSystemLibrary.IsValid` _hitcomponent) (`ActorComponent.ComponentHasTag` _hitcomponent "Item"))
      (set `self.ItemName` (`KismetSystemLibrary.GetDisplayName` _hitcomponent))
      (`self.EnableInput` _returnvalue)
      (`WidgetBlueprintLibrary.SetInputMode_GameOnly` _returnvalue)
      (return)
      (else
        (return)))
    (else
      (return))))

(fn `UserConstructionScript`
  ;[1 1 1] Creates a dynamic material for the right/wrong light
  (bind _returnvalue (`PrimitiveComponent.CreateDynamicMaterialInstance` (`self.Keypad`) 0 "/Game/PadlockAndKeypadPack/Keypad/Materials/M_Keypad_Red.M_Keypad_Red" "None"))
  (set `self.KeypadMaterialWrong` _returnvalue)
  (bind _returnvalue_2 (`PrimitiveComponent.CreateDynamicMaterialInstance` (`self.Keypad`) 0 "/Game/PadlockAndKeypadPack/Keypad/Materials/M_Keypad_Green.M_Keypad_Green" "None"))
  (set `self.KeypadMaterialRight` _returnvalue_2)
  ;[1 1 1] Sets the transform of the camera
  (`SceneComponent.K2_AddLocalTransform` (`self.Camera`) (`self.CameraTransform`) false false)
  ;[1 1 1] Sets a random code
  (if (`self.RandomCode?`)
    (set `self.Code` (`KismetStringLibrary.Conv_IntToString` (`KismetMathLibrary.RandomIntegerInRange` 1000 9999)))
    (set `self.CodeLength` 4)
    (else
      (set `self.CodeLength` (`KismetStringLibrary.Len` (`self.Code`)))))
  (if (`self.TurnOffText?`)
    (`SceneComponent.SetHiddenInGame` (`self.TextRender`) true false)
    (else
      (`TextRenderComponent.K2_SetText` (`self.TextRender`) (`KismetTextLibrary.Conv_StringToText` (`self.Code`)))))
  (for (_array_element _array_index) (`|MakeArray` (`self.Keypad`) (`self.0`) (`self.1`) (`self.2`) (`self.3`) (`self.4`) (`self.5`) (`self.6`) (`self.7`) (`self.8`) (`self.9`) (`self.Clear`) (`self.Enter`))
    (`KismetArrayLibrary.Array_Set` (`self.KeypadNamesArray`) _array_index (`KismetSystemLibrary.GetDisplayName` _array_element) true)))