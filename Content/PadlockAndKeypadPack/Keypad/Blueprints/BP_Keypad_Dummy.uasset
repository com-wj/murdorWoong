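; Keypad actor that builds a fixed or random four-digit code, optionally shown on a text render.
; Construction also creates red and green light materials and caches component names.
; Cursor hover toggles input, and F applies negligible damage to itself, with no damage handler here.
; Helper functions for clearing entry, switching player input and camera tracing for "Item"-tagged components are defined but never called here.
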(event `self.ReceiveActorBeginCursorOver`
  (`self.EnableInput` (`GameplayStatics.GetPlayerController` 0)))

(event `self.ReceiveActorEndCursorOver`
  (`self.DisableInput` (`GameplayStatics.GetPlayerController` 0)))

(event `Key|F`
  (params (Key :type "Key Structure"))
  (:`Pressed`
    (`GameplayStatics.ApplyDamage` self 0.0001)))

(fn `ClearCode`
  ;[1 1 1] Resets the code when the clear button is pressed
  (`KismetArrayLibrary.Array_Clear` (`self.EnteredCode`))
  (set `self.CodeString` "")
  (return))

(fn `Enable/DisablePlayerInput`
  (params (`Enable?` :type Boolean))
  (if `Enable?`
    (`self.EnableInput` (`GameplayStatics.GetPlayerCharacter` 0) (`GameplayStatics.GetPlayerController` 0))
    (`self.DisableInput` (`GameplayStatics.GetPlayerController` 0))
    (else
      (`self.DisableInput` (`GameplayStatics.GetPlayerCharacter` 0) (`GameplayStatics.GetPlayerController` 0)))))

(fn `LineTraceForKeypad`
  (locals (TraceStartLocation :type "Vector Structure") (TraceEndLocation :type "Vector Structure"))
  (bind _returnvalue (`GameplayStatics.GetPlayerController` 0))
  (bind _output (`|GetArrayItem` (`self.K2_GetComponentsByClass` (`GameplayStatics.GetPlayerCharacter` 0) "/Script/Engine.CameraComponent")))
  (bind _returnvalue_2 (`SceneComponent.K2_GetComponentLocation` _output))
  (set `local.TraceStartLocation` _returnvalue_2)
  (set `local.TraceEndLocation` (+ _returnvalue_2 (* (`SceneComponent.GetForwardVector` _output) 250.0)))
  (set `self.ItemName` "")
  (bind (_outhit _returnvalue_3) (`KismetSystemLibrary.LineTraceSingle` :`Start` (`local.TraceStartLocation`) :`End` (`local.TraceEndLocation`) :`TraceChannel` "TraceTypeQuery1" :`bIgnoreSelf` false))
  (if _returnvalue_3
    (bind (_bblockinghit _binitialoverlap _time _distance _location _impactpoint _normal _impactnormal _physmat _hitactor _hitcomponent) (`GameplayStatics.BreakHitResult` _outhit))
    (if (and (`KismetSystemLibrary.IsValid` _hitcomponent) (`ActorComponent.ComponentHasTag` _hitcomponent "Item"))
      (set `self.ItemName` (`KismetSystemLibrary.GetDisplayName` _hitcomponent))
      (`self.EnableInput` _returnvalue)
      (`WidgetBlueprintLibrary.SetInputMode_GameOnly` _returnvalue)
      (return)
      (else
        (return)))
    (else
      (return))))

(fn `UserConstructionScript`
  ;[1 1 1] Creates a dynamic material for the right/wrong light
  (bind _returnvalue (`PrimitiveComponent.CreateDynamicMaterialInstance` (`self.Keypad`) 0 "/Game/PadlockAndKeypadPack/Keypad/Materials/M_Keypad_Red.M_Keypad_Red" "None"))
  (set `self.KeypadMaterialWrong` _returnvalue)
  (bind _returnvalue_2 (`PrimitiveComponent.CreateDynamicMaterialInstance` (`self.Keypad`) 0 "/Game/PadlockAndKeypadPack/Keypad/Materials/M_Keypad_Green.M_Keypad_Green" "None"))
  (set `self.KeypadMaterialRight` _returnvalue_2)
  ;[1 1 1] Sets a random code
  (if (`self.RandomCode?`)
    (set `self.Code` (`KismetStringLibrary.Conv_IntToString` (`KismetMathLibrary.RandomIntegerInRange` 1000 9999)))
    (set `self.CodeLength` 4)
    (else
      (set `self.CodeLength` (`KismetStringLibrary.Len` (`self.Code`)))))
  (if (`self.TurnOffText?`)
    (`SceneComponent.SetHiddenInGame` (`self.TextRender`) true false)
    (else
      (`TextRenderComponent.K2_SetText` (`self.TextRender`) (`KismetTextLibrary.Conv_StringToText` (`self.Code`)))))
  (for (_array_element _array_index) (`|MakeArray` (`self.Keypad`) (`self.0`) (`self.1`) (`self.2`) (`self.3`) (`self.4`) (`self.5`) (`self.6`) (`self.7`) (`self.8`) (`self.9`) (`self.Clear`) (`self.Enter`))
    (`KismetArrayLibrary.Array_Set` (`self.KeypadNamesArray`) _array_index (`KismetSystemLibrary.GetDisplayName` _array_element) true)))