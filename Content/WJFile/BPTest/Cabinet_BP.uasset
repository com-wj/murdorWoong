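; Interactive cabinet Blueprint with separate top and bottom pairs of doors that the player opens and closes with F.
; Cursor hover over door or box components enables player input and records whether the top or bottom section is targeted; leaving disables input.
; A FlipFlop per section alternates playing and reversing its timeline, which swings the left and right doors to mirrored yaw angles scaled by MaxAngle.
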(event `self.Door_Top_Left.OnBeginCursorOver`
  (params (TouchedComponent :type "PrimitiveComponent Object Reference"))
  (set `self.aimtotop` true :!label _label)
  (`self.EnableInput` (`GameplayStatics.GetPlayerController` 0) :!label _label_2))

(event `self.Door_Top_Right.OnBeginCursorOver`
  (params (TouchedComponent :type "PrimitiveComponent Object Reference"))
  (goto _label))

(event `self.topbox.OnBeginCursorOver`
  (params (TouchedComponent :type "PrimitiveComponent Object Reference"))
  (goto _label))

(event `self.topleftbox.OnBeginCursorOver`
  (params (TouchedComponent :type "PrimitiveComponent Object Reference"))
  (goto _label))

(event `self.toprightbox.OnBeginCursorOver`
  (params (TouchedComponent :type "PrimitiveComponent Object Reference"))
  (goto _label))

(event `self.Door_Bottom_Left.OnBeginCursorOver`
  (params (TouchedComponent :type "PrimitiveComponent Object Reference"))
  (set `self.aimtotop` false :!label _label_3)
  (goto _label_2))

(event `self.Door_Bottom_Right.OnBeginCursorOver`
  (params (TouchedComponent :type "PrimitiveComponent Object Reference"))
  (goto _label_3))

(event `self.bottombox.OnBeginCursorOver`
  (params (TouchedComponent :type "PrimitiveComponent Object Reference"))
  (goto _label_3))

(event `self.bottomleftbox.OnBeginCursorOver`
  (params (TouchedComponent :type "PrimitiveComponent Object Reference"))
  (goto _label_3))

(event `Key|F`
  (params (Key :type "Key Structure"))
  (:`Pressed`
    (if (`self.aimtotop`)
      (`/Engine/EditorBlueprintResources/StandardMacros.FlipFlop`
        (:`A`
          (`self.Open`))
        (:`B`
          (`self.Close`)))
      (else
        (`/Engine/EditorBlueprintResources/StandardMacros.FlipFlop`
          (:`A`
            (`self.Open_Bottom`))
          (:`B`
            (`self.Close_Bottom`)))))))

(event `self.bottomrightbox.OnBeginCursorOver`
  (params (TouchedComponent :type "PrimitiveComponent Object Reference"))
  (goto _label_3))

(event `self.Door_Bottom_Right.OnEndCursorOver`
  (params (TouchedComponent :type "PrimitiveComponent Object Reference"))
  (`self.DisableInput` (`GameplayStatics.GetPlayerController` 0) :!label _label_4))

(event `self.Door_Bottom_Left.OnEndCursorOver`
  (params (TouchedComponent :type "PrimitiveComponent Object Reference"))
  (goto _label_4))

(event `self.Door_Top_Left.OnEndCursorOver`
  (params (TouchedComponent :type "PrimitiveComponent Object Reference"))
  (goto _label_4))

(event `self.Door_Top_Right.OnEndCursorOver`
  (params (TouchedComponent :type "PrimitiveComponent Object Reference"))
  (goto _label_4))

(event `self.topbox.OnEndCursorOver`
  (params (TouchedComponent :type "PrimitiveComponent Object Reference"))
  (goto _label_4))

(event `self.bottombox.OnEndCursorOver`
  (params (TouchedComponent :type "PrimitiveComponent Object Reference"))
  (goto _label_4))

(event `self.topleftbox.OnEndCursorOver`
  (params (TouchedComponent :type "PrimitiveComponent Object Reference"))
  (goto _label_4))

(event `self.toprightbox.OnEndCursorOver`
  (params (TouchedComponent :type "PrimitiveComponent Object Reference"))
  (goto _label_4))

(event `self.bottomleftbox.OnEndCursorOver`
  (params (TouchedComponent :type "PrimitiveComponent Object Reference"))
  (goto _label_4))

(event `self.bottomrightbox.OnEndCursorOver`
  (params (TouchedComponent :type "PrimitiveComponent Object Reference"))
  (goto _label_4))

(event `Open`
  (bind _maxangle (`self.MaxAngle`))
  ;[1 1 1] 윗문 열기
  (bind (_direction _angle) (`Timeline|OpeningTop` :!label _label_5)
    (:`Update`
      (bind _returnvalue (* _maxangle _angle))
      (if (<= _returnvalue _maxangle)
        (`SceneComponent.K2_SetRelativeRotation` (`self.Door_Top_Left`) (`KismetMathLibrary.MakeRotator` 0.0 0.0 _returnvalue) false false)
        (`SceneComponent.K2_SetRelativeRotation` (`self.Door_Top_Right`) (`KismetMathLibrary.MakeRotator` 0.0 0.0 (* _returnvalue -1.0)) false false)))))

(event `Close`
  ;[1 1 1] 윗문 열기
  (goto _label_5 :!via `Reverse`))

(event `Open_Bottom`
  (bind _maxangle (`self.MaxAngle`))
  ;[1 1 1] 아랫문 열기
  (bind (_direction _angle) (`Timeline|OpeningBottom` :!label _label_6)
    (:`Update`
      (bind _returnvalue (* _maxangle _angle))
      (if (<= _returnvalue _maxangle)
        (`SceneComponent.K2_SetRelativeRotation` (`self.Door_Bottom_Left`) (`KismetMathLibrary.MakeRotator` 0.0 0.0 _returnvalue) false false)
        (`SceneComponent.K2_SetRelativeRotation` (`self.Door_Bottom_Right`) (`KismetMathLibrary.MakeRotator` 0.0 0.0 (* _returnvalue -1.0)) false false)))))

(event `Close_Bottom`
  ;[1 1 1] 아랫문 열기
  (goto _label_6 :!via `Reverse`))

(fn `UserConstructionScript`)