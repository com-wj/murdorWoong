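; Dummy box head actor that the player swings open and closed with the F key while the cursor is over its mesh.
; Cursor hover events toggle input on the actor, and BeginPlay caches the actor's starting location and rotation.
; F plays a drawer sound, then a FlipFlop eases the mesh between a rolled pose and the cached one, using a DoOnce to gate repeat presses.
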(event `self.StaticMeshComponent.OnBeginCursorOver`
  (params (TouchedComponent :type "PrimitiveComponent Object Reference"))
  (`self.EnableInput` (`GameplayStatics.GetPlayerController` 0)))

(event `self.ReceiveBeginPlay`
  (bind (_returnvalue_location _returnvalue_rotation) (`KismetMathLibrary.BreakTransform` (`self.GetTransform`)))
  (set `self.default coordinate` _returnvalue_location)
  (set `self.Default Rotate` _returnvalue_rotation))

(event `self.StaticMeshComponent.OnEndCursorOver`
  (params (TouchedComponent :type "PrimitiveComponent Object Reference"))
  (`self.DisableInput` (`GameplayStatics.GetPlayerController` 0)))

(event `Key|F`
  (params (Key :type "Key Structure"))
  (bind _staticmeshcomponent (`self.StaticMeshComponent`))
  (bind (_default_rotate_roll _default_rotate_pitch _default_rotate_yaw) (`KismetMathLibrary.BreakRotator` (`self.Default Rotate`)))
  (bind _default_coordinate (`self.default coordinate`))
  (:`Pressed`
    (cast `/Game/FirstPersonBP/Blueprints/FirstPersonCharacter` (`GameplayStatics.GetPlayerCharacter` 0))
    (`/Engine/EditorBlueprintResources/StandardMacros.DoOnce` false :!label _label
      (:`Completed`
        (`GameplayStatics.PlaySound2D` "/Game/sound/se/se_drawer_move.se_drawer_move" 1.0 1.0 0.5 null null)
        (`/Engine/EditorBlueprintResources/StandardMacros.FlipFlop`
          (:`A`
            (`KismetSystemLibrary.MoveComponentTo` _staticmeshcomponent _default_coordinate (`KismetMathLibrary.MakeRotator` (+ _default_rotate_roll -100.0) _default_rotate_pitch _default_rotate_yaw) false true 1.0)
            (goto _label :!via `Reset`))
          (:`B`
            (`KismetSystemLibrary.MoveComponentTo` _staticmeshcomponent _default_coordinate (`KismetMathLibrary.MakeRotator` _default_rotate_roll _default_rotate_pitch _default_rotate_yaw) false true 1.0)
            (goto _label :!via `Reset`)))))))

(fn `UserConstructionScript`)