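; Interactable murder diary prop that the player reads by pressing F while the cursor is over its mesh.
; Cursor-over events on the static mesh enable and disable the actor's input, so the key only responds during hover.
; The first press sets TextMsgNum on the cached FirstPersonCharacter and marks the diary as read.
; The F handler also applies a negligible amount of damage to the diary itself, with no damage handler in this graph.
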(event `self.StaticMeshComponent.OnBeginCursorOver`
  (params (TouchedComponent :type "PrimitiveComponent Object Reference"))
  (`self.EnableInput` (`GameplayStatics.GetPlayerController` 0)))

(event `self.StaticMeshComponent.OnEndCursorOver`
  (params (TouchedComponent :type "PrimitiveComponent Object Reference"))
  (`self.DisableInput` (`GameplayStatics.GetPlayerController` 0)))

(event `Key|F`
  (params (Key :type "Key Structure"))
  (:`Pressed`
    (if (not (`self.Diary Read`))
      (set `/Game/FirstPersonBP/Blueprints/FirstPersonCharacter.text msg Num` 3 (stale `self.ReceiveBeginPlay` _asfirst_person_character))
      (set `self.Diary Read` true))
    (`GameplayStatics.ApplyDamage` self 0.0001)))

(event `self.ReceiveBeginPlay`
  (bind _asfirst_person_character (cast `/Game/FirstPersonBP/Blueprints/FirstPersonCharacter` (`GameplayStatics.GetPlayerCharacter` 0))))

(fn `UserConstructionScript`)