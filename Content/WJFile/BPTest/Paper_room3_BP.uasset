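; Paper_room3_BP is a note actor, apparently for room 3, that the player marks as read by pressing F while hovering over it.
; Cursor-over events on its mesh enable and disable the actor's input.
; F sets Note3Read on the FirstPersonCharacter if unset, then applies negligible damage to the paper itself on every press, with no damage handler in this Blueprint.
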(event `self.StaticMeshComponent.OnBeginCursorOver`
  (params (TouchedComponent :type "PrimitiveComponent Object Reference"))
  (`self.EnableInput` (`GameplayStatics.GetPlayerController` 0)))

(event `self.StaticMeshComponent.OnEndCursorOver`
  (params (TouchedComponent :type "PrimitiveComponent Object Reference"))
  (`self.DisableInput` (`GameplayStatics.GetPlayerController` 0)))

(event `Key|F`
  (params (Key :type "Key Structure"))
  (:`Pressed`
    (bind _asfirst_person_character (cast `/Game/FirstPersonBP/Blueprints/FirstPersonCharacter` (`GameplayStatics.GetPlayerCharacter` 0)))
    (if (not (`/Game/FirstPersonBP/Blueprints/FirstPersonCharacter.note 3 read` _asfirst_person_character))
      (set `/Game/FirstPersonBP/Blueprints/FirstPersonCharacter.note 3 read` true _asfirst_person_character))
    (`GameplayStatics.ApplyDamage` self 0.0001)))

(fn `UserConstructionScript`)