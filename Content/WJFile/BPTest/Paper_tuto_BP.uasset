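; Note item pickup actor, apparently for a tutorial, collected by hovering the cursor over it and pressing F.
; The static mesh's cursor-over events enable and disable the actor's input for player controller 0.
; On F it sets the first note flag (ItemNote1Have) on the GI_Woong game instance cached at BeginPlay, plays the item-get sound and destroys itself.
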(event `self.StaticMeshComponent.OnBeginCursorOver`
  (params (TouchedComponent :type "PrimitiveComponent Object Reference"))
  (`self.EnableInput` (`GameplayStatics.GetPlayerController` 0)))

(event `self.StaticMeshComponent.OnEndCursorOver`
  (params (TouchedComponent :type "PrimitiveComponent Object Reference"))
  (`self.DisableInput` (`GameplayStatics.GetPlayerController` 0)))

(event `Key|F`
  (params (Key :type "Key Structure"))
  (:`Pressed`
    (set `/Game/GI_Woong.item_note 1 have` true (stale `self.ReceiveBeginPlay` _asgi_woong))
    (`GameplayStatics.PlaySound2D` "/Game/sound/se/se_itemGet.se_itemGet" 1.0 1.0 0.05 null null) ; 아이템 획득 사운드
    (`self.K2_DestroyActor`)))

(event `self.ReceiveBeginPlay`
  (bind _asgi_woong (cast `/Game/GI_Woong` (`GameplayStatics.GetGameInstance`))))

(fn `UserConstructionScript`)