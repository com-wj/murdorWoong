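; A wall trigger box that responds to the F key while the cursor is over it.
; Cursor over and out events on its collision component toggle input from the player controller.
; Pressing F sets the first-person character's TextMsgNum to a fixed message while Firsttouch is false, a flag the level blueprint controls.
; Each press also applies negligible damage to itself.
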(event `self.CollisionComponent.OnBeginCursorOver`
  (params (TouchedComponent :type "PrimitiveComponent Object Reference"))
  (`self.EnableInput` (`GameplayStatics.GetPlayerController` 0)))

(event `self.CollisionComponent.OnEndCursorOver`
  (params (TouchedComponent :type "PrimitiveComponent Object Reference"))
  (`self.DisableInput` (`GameplayStatics.GetPlayerController` 0)))

(event `Key|F`
  (params (Key :type "Key Structure"))
  (:`Pressed`
    (if (not (`self.firsttouch`))
      (set `/Game/FirstPersonBP/Blueprints/FirstPersonCharacter.text msg Num` 6 (stale `self.ReceiveBeginPlay` _asfirst_person_character)))
    (`GameplayStatics.ApplyDamage` self 0.0001)))

(event `self.ReceiveBeginPlay`
  (bind _asfirst_person_character (cast `/Game/FirstPersonBP/Blueprints/FirstPersonCharacter` (`GameplayStatics.GetPlayerCharacter` 0))))

(fn `UserConstructionScript`)