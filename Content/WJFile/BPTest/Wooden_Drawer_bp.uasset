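; Interactive wooden drawer that slides open and shut and holds a collectible key.
; Cursor hover enables input, so F either toggles the drawer via a DoOnce-guarded FlipFlop and MoveComponentTo, or takes the key when aimed at its box.
; Pickup sets the first-person character's key flag and message number, applies token self-damage and destroys key and box.
; After a short BeginPlay delay, NotLevel1 also removes the key and box.
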(event `self.StaticMeshComponent.OnBeginCursorOver`
  (params (TouchedComponent :type "PrimitiveComponent Object Reference"))
  (`self.EnableInput` (`GameplayStatics.GetPlayerController` 0)))

(event `self.StaticMeshComponent.OnEndCursorOver`
  (params (TouchedComponent :type "PrimitiveComponent Object Reference"))
  (`self.DisableInput` (`GameplayStatics.GetPlayerController` 0)))

(event `self.Box.OnBeginCursorOver`
  (params (TouchedComponent :type "PrimitiveComponent Object Reference"))
  (`self.EnableInput` (`GameplayStatics.GetPlayerController` 0))
  (set `self.AimToItem` true))

(event `self.Box.OnEndCursorOver`
  (params (TouchedComponent :type "PrimitiveComponent Object Reference"))
  (`self.DisableInput` (`GameplayStatics.GetPlayerController` 0))
  (set `self.AimToItem` false))

(event `Key|F`
  (params (Key :type "Key Structure"))
  (bind _staticmeshcomponent (`self.StaticMeshComponent`))
  (bind (_default_coordinate_x _default_coordinate_y _default_coordinate_z) (`KismetMathLibrary.BreakVector` (`self.default coordinate`)))
  (bind _default_rotate (`self.Default Rotate`))
  (:`Pressed`
    (if (`self.AimToItem`)
      (set `/Game/FirstPersonBP/Blueprints/FirstPersonCharacter.item_key 1 have` true (stale `self.ReceiveBeginPlay` _asfirst_person_character))
      (set `/Game/FirstPersonBP/Blueprints/FirstPersonCharacter.block msg Num` 3 (stale `self.ReceiveBeginPlay` _asfirst_person_character))
      (`GameplayStatics.PlaySound2D` "/Game/sound/se/se_itemGet.se_itemGet" 1.0 1.0 0.05 null null)
      (`GameplayStatics.ApplyDamage` self 0.0001)
      (`ActorComponent.K2_DestroyComponent` (`self.Key`))
      (`ActorComponent.K2_DestroyComponent` (`self.Box`))
      (set `self.AimToItem` false)
      (else
        (`/Engine/EditorBlueprintResources/StandardMacros.DoOnce` false :!label _label
          (:`Completed`
            (`GameplayStatics.PlaySound2D` "/Game/sound/se/se_drawer_move.se_drawer_move" 1.0 1.0 0.5 null null)
            (`/Engine/EditorBlueprintResources/StandardMacros.FlipFlop`
              (:`A`
                (`KismetSystemLibrary.MoveComponentTo` _staticmeshcomponent (`KismetMathLibrary.MakeVector` _default_coordinate_x (+ _default_coordinate_y -35.0) _default_coordinate_z) _default_rotate false true 0.9)
                (goto _label :!via `Reset`))
              (:`B`
                (`KismetSystemLibrary.MoveComponentTo` _staticmeshcomponent (`KismetMathLibrary.MakeVector` _default_coordinate_x _default_coordinate_y _default_coordinate_z) _default_rotate false false 0.9)
                (goto _label :!via `Reset`)))))))))

(event `self.ReceiveBeginPlay`
  (bind (_returnvalue_location _returnvalue_rotation) (`KismetMathLibrary.BreakTransform` (`self.GetTransform`)))
  (set `self.default coordinate` _returnvalue_location)
  (set `self.Default Rotate` _returnvalue_rotation)
  (bind _asfirst_person_character (cast `/Game/FirstPersonBP/Blueprints/FirstPersonCharacter` (`GameplayStatics.GetPlayerCharacter` 0)))
  (`KismetSystemLibrary.Delay` 1.0)
  (if (`self.NotLevel1`)
    (`ActorComponent.K2_DestroyComponent` (`self.Key`))
    (`ActorComponent.K2_DestroyComponent` (`self.Box`))))

(fn `UserConstructionScript`)