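; Room 4 key pickup actor that the first-person player collects by pointing the cursor at it and pressing F.
; Cursor hover over its static mesh or box enables input on the actor, and leaving disables it.
; F sets the item-key-4 flag and a message number on the character cached at BeginPlay, plays a pickup sound, applies negligible damage to itself, then destroys the actor.
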(event `self.StaticMeshComponent.OnBeginCursorOver`
  (params (TouchedComponent :type "PrimitiveComponent Object Reference"))
  (`self.EnableInput` (`GameplayStatics.GetPlayerController` 0) :!label _label))

(event `self.Box.OnBeginCursorOver`
  (params (TouchedComponent :type "PrimitiveComponent Object Reference"))
  (goto _label))

(event `self.StaticMeshComponent.OnEndCursorOver`
  (params (TouchedComponent :type "PrimitiveComponent Object Reference"))
  (`self.DisableInput` (`GameplayStatics.GetPlayerController` 0) :!label _label_2))

(event `self.Box.OnEndCursorOver`
  (params (TouchedComponent :type "PrimitiveComponent Object Reference"))
  (goto _label_2))

(event `Key|F`
  (params (Key :type "Key Structure"))
  (:`Pressed`
    (set `/Game/FirstPersonBP/Blueprints/FirstPersonCharacter.item_key 4 have` true (stale `self.ReceiveBeginPlay` _asfirst_person_character))
    (set `/Game/FirstPersonBP/Blueprints/FirstPersonCharacter.block msg Num` 5 (stale `self.ReceiveBeginPlay` _asfirst_person_character))
    (`GameplayStatics.PlaySound2D` "/Game/sound/se/se_itemGet.se_itemGet" 1.0 1.0 0.05 null null)
    (`GameplayStatics.ApplyDamage` self 0.0001)
    (`self.K2_DestroyActor`)))

(event `self.ReceiveBeginPlay`
  (bind _asfirst_person_character (cast `/Game/FirstPersonBP/Blueprints/FirstPersonCharacter` (`GameplayStatics.GetPlayerCharacter` 0))))

(fn `UserConstructionScript`)