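; Cuttable chain that the first-person player breaks with F when carrying the cutter item.
; Cursor hover over the mesh or box enables actor input, and leaving disables it.
; Cutting plays a sound, turns on gravity, blocks further interaction through the Visibility channel, then destroys the chain after a delay.
; Without the cutter it sets the character's message number; both outcomes apply negligible damage to itself.
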(event `self.StaticMeshComponent.OnBeginCursorOver`
  (params (TouchedComponent :type "PrimitiveComponent Object Reference"))
  (`self.EnableInput` (`GameplayStatics.GetPlayerController` 0) :!label _label))

(event `self.Box.OnBeginCursorOver`
  (params (TouchedComponent :type "PrimitiveComponent Object Reference"))
  (goto _label))

(event `self.StaticMeshComponent.OnEndCursorOver`
  (params (TouchedComponent :type "PrimitiveComponent Object Reference"))
  (`self.DisableInput` (`GameplayStatics.GetPlayerController` 0) :!label _label_2))

(event `self.Box.OnEndCursorOver`
  (params (TouchedComponent :type "PrimitiveComponent Object Reference"))
  (goto _label_2))

(event `Key|F`
  (params (Key :type "Key Structure"))
  (bind _staticmeshcomponent (`self.StaticMeshComponent`))
  (:`Pressed`
    (if (`/Game/FirstPersonBP/Blueprints/FirstPersonCharacter.item_cutter have` (stale `self.ReceiveBeginPlay` _asfirst_person_character))
      (`GameplayStatics.PlaySound2D` "/Game/sound/se/se_chain_cut.se_chain_cut" 1.0 1.0 0.3 null null) ; 사슬 끊는 소리
      (`PrimitiveComponent.SetEnableGravity` _staticmeshcomponent true)
      (`PrimitiveComponent.SetCollisionResponseToChannel` _staticmeshcomponent "ECC_Visibility" "ECR_Overlap") ; 더이상 상호작용 불가
      (`GameplayStatics.ApplyDamage` self 0.0001)
      (`KismetSystemLibrary.Delay` 5.0)
      (`self.K2_DestroyActor`)
      (else
        (set `/Game/FirstPersonBP/Blueprints/FirstPersonCharacter.text msg Num` 5 (stale `self.ReceiveBeginPlay` _asfirst_person_character))
        (`GameplayStatics.ApplyDamage` self 0.0001)
        (`KismetSystemLibrary.PrintText` "체인박스 터치")))))

(event `self.ReceiveBeginPlay`
  (bind _asfirst_person_character (cast `/Game/FirstPersonBP/Blueprints/FirstPersonCharacter` (`GameplayStatics.GetPlayerCharacter` 0))))

(fn `UserConstructionScript`)